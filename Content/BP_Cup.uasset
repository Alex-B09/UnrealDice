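; Dice cup actor that spawns, shakes and throws BP_D6 dice.
; On BeginPlay it spawns two batches of four dice at scene-component points, a second apart, storing them in Dices.
; A looping timer keeps them jostling with random-strength radial impulses from inside the cup.
; Throw stops the timer and plays a timeline that rolls the cup mesh, disables cover collision and fires a final velocity-change impulse at the dice.
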(event `self.ReceiveBeginPlay`
  (`|ExecutionSequence`
    (:`then_0`
      (`self.SpawnDices`)
      (`KismetSystemLibrary.Delay` 1.0)
      (`self.SpawnDices`))
    (:`then_1`
      (set `self.Popper` (`|MakeArray` (`self.Scene`) (`self.Scene1`) (`self.Scene2`) (`self.Scene3`) (`self.Scene4`)))
      (bind _returnvalue (`KismetSystemLibrary.K2_SetTimerDelegate` (delegate `AddPop`) 0.5 true 1.5))
      (set `self.Timer` _returnvalue))))

(event `AddPop`
  (for _array_element (`self.Dices`)
    (`KismetSystemLibrary.PrintString` "Hello")
    (`PrimitiveComponent.AddRadialImpulse` (`/Game/BP_D6.Mesh` _array_element) (`SceneComponent.K2_GetComponentLocation` (`self.Scene`)) 200.0 (`KismetMathLibrary.RandomFloatInRange` 3000.0 5000.0) "RIF_Linear" false)))

(event `Throw`
  (`KismetSystemLibrary.PrintString` "121212121221" true true (struct :`R` 1.0 :`G` 0.22762 :`B` 0.357605 :`A` 1.0))
  (`KismetSystemLibrary.K2_ClearAndInvalidateTimerHandle` (`self.Timer`))
  (bind (_direction _turnrate) (`Timeline|TurnRate` :!via `PlayFromStart`)
    (:`Update`
      (`SceneComponent.K2_SetRelativeRotation` (`self.StaticMesh`) (`KismetMathLibrary.MakeRotator` (* _turnrate 140.0)) false false))
    (:`PrepareForRelease`
      (`PrimitiveComponent.SetCollisionEnabled` (`self.Cover`) "NoCollision"))
    (:`FinalPop`
      (for _array_element (`self.Dices`)
        (`PrimitiveComponent.AddRadialImpulse` (`/Game/BP_D6.Mesh` _array_element) (`SceneComponent.K2_GetComponentLocation` (`self.Scene`)) 1000.0 750.0 "RIF_Constant" true)))))

(fn `SpawnDices`
  (`|ExecutionSequence`
    (:`then_0`
      (bind _returnvalue (`|SpawnActorFromClass` "/Game/BP_D6.BP_D6_C" (`SceneComponent.K2_GetComponentToWorld` (`self.Scene1`)) "Undefined" "OverrideRootScale" self null))
      (`KismetArrayLibrary.Array_Add` (`self.Dices`) _returnvalue))
    (:`then_1`
      (bind _returnvalue_2 (`|SpawnActorFromClass` "/Game/BP_D6.BP_D6_C" (`SceneComponent.K2_GetComponentToWorld` (`self.Scene2`)) "Undefined" "OverrideRootScale" self null))
      (`KismetArrayLibrary.Array_Add` (`self.Dices`) _returnvalue_2))
    (:`then_2`
      (bind _returnvalue_3 (`|SpawnActorFromClass` "/Game/BP_D6.BP_D6_C" (`SceneComponent.K2_GetComponentToWorld` (`self.Scene3`)) "Undefined" "OverrideRootScale" self null))
      (`KismetArrayLibrary.Array_Add` (`self.Dices`) _returnvalue_3))
    (:`then_3`
      (bind _returnvalue_4 (`|SpawnActorFromClass` "/Game/BP_D6.BP_D6_C" (`SceneComponent.K2_GetComponentToWorld` (`self.Scene4`)) "Undefined" "OverrideRootScale" self null))
      (`KismetArrayLibrary.Array_Add` (`self.Dices`) _returnvalue_4))))

(fn `UserConstructionScript`)